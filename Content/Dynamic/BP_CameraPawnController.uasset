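; Controller for BP_CameraPawn that toggles the camera between a first-person mode and a spring-arm mode.
; On BeginPlay it caches the player pawn and its initial spring arm length.
; The SwitchCameraMode input collapses or extends the arm and shifts the pawn's Sphere backward or forward along its forward vector by the cached length.
; Extending uses a hard-coded arm length instead of the cached one.
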(event EventBeginPlay
  (Utilities|FlowControl|Sequence
    (:then_0
      (bind _asbp_camera_pawn (Utilities|Casting|CastToBP_CameraPawn (Game|Player|GetPlayerPawn 0)))
      (bind _output_get (Variables|References|SetCameraPawnRef _asbp_camera_pawn))
      (Variables|References|SetCameraTargetArmLengthRef (Variables|/Script/Engine.SpringArmComponent|GetTargetArmLength (Variables|/Game/Dynamic/BP_CameraPawn.BP_CameraPawn_C|GetSpringArm _output_get))))))

(event EventTick
  (params (DeltaSeconds :type Float%20%28single-precision%29)))

(event Input|ActionEvents|InputActionSwitchCameraMode
  (params (Key :type Key%20Structure))
  (bind _camerapawnref (Variables|References|GetCameraPawnRef))
  (bind _springarm (Variables|/Game/Dynamic/BP_CameraPawn.BP_CameraPawn_C|GetSpringArm _camerapawnref))
  (bind _sphere (Variables|/Game/Dynamic/BP_CameraPawn.BP_CameraPawn_C|GetSphere _camerapawnref))
  (bind _sphere_2 (Variables|/Game/Dynamic/BP_CameraPawn.BP_CameraPawn_C|GetSphere _camerapawnref))
  (:Pressed
    (bind _output_get (Variables|Default|SetbFirstPerson (not (Variables|Default|GetbFirstPerson))))
    (if _output_get
      (Variables|/Script/Engine.SpringArmComponent|SetTargetArmLength _springarm 0.0)
      (Transformation|SetWorldLocation _sphere_2 (- (Transformation|GetWorldLocation _sphere_2) (* (Math|Vector|GetForwardVector _sphere_2) (Variables|References|GetCameraTargetArmLengthRef))) false false)
      (else
        (Variables|/Script/Engine.SpringArmComponent|SetTargetArmLength _springarm 1e+03)
        (Transformation|SetWorldLocation _sphere (+ (Transformation|GetWorldLocation _sphere) (* (Math|Vector|GetForwardVector _sphere) (Variables|References|GetCameraTargetArmLengthRef))) false false)))))

(fn ConstructionScript)