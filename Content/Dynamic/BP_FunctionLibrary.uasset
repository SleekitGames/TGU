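; BP_FunctionLibrary is a Blueprint function library for finding what lies directly beneath a given actor.
; Both functions line trace straight down 100,000 units from the actor's location, returning the hit actor and its distance as a vertical offset.
; GetTerrainBlockBelowActor uses a custom trace channel to find terrain blocks.
; GetObjectBelowActor traces on Visibility and also returns whether anything was hit.
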(fn GetTerrainBlockBelowActor
  (params (Actor :type Actor%20Object%20Reference))
  (bind _returnvalue (Transformation|GetActorLocation Actor))
  (bind (_x _y _z) (Math|Vector|BreakVector _returnvalue))
  (bind _outhit (Collision|LineTraceByChannel Actor _returnvalue (Math|Vector|MakeVector _x _y (- _z 1e+05)) "TraceTypeQuery3" false 0 "None"))
  (return (.hitactor _outhit) (.distance _outhit)))

(fn GetObjectBelowActor
  (params (Actor :type Actor%20Object%20Reference))
  (bind _returnvalue (Transformation|GetActorLocation Actor))
  (bind (_x _y _z) (Math|Vector|BreakVector _returnvalue))
  (bind (_outhit _returnvalue_2) (Collision|LineTraceByChannel Actor _returnvalue (Math|Vector|MakeVector _x _y (- _z 1e+05)) "TraceTypeQuery1" false 0 "None"))
  (return (.hitactor _outhit) (.distance _outhit) _returnvalue_2))