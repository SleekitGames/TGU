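; Grid selection actor that previews a drag-selected building footprint and spawns BP_Foundations at its minimum corner.
; GridClickStart opens a Tick gate that stretches HoverMesh between the start point and cursor hit, snapped using the GameMode's GridSize.
; Overlap events track blocking actors to set Buildable, which switches the preview material.
; GridClickEnd computes square counts, spawns and closes the gate, or prints an error if invalid.
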(event Custom|GridClickStart
  (bind _gamemoderef (Variables|Default|GetGameModeRef))
  (bind _camerapawncontrollerref (Variables|Default|GetCameraPawnControllerRef))
  (bind _gamemoderef_2 (Variables|Default|GetGameModeRef))
  (bind _camerapawncontrollerref_2 (Variables|Default|GetCameraPawnControllerRef))
  (bind _hitresult (Game|Player|GetHitResultUnderCursorbyChannel _camerapawncontrollerref "TraceTypeQuery4" false))
  (bind _gridsize (Variables|/Game/Dynamic/BP_TGUGameMode.BP_TGUGameMode_C|GetGridSize _gamemoderef))
  (bind _gridsize_2 (Variables|/Game/Dynamic/BP_TGUGameMode.BP_TGUGameMode_C|GetGridSize _gamemoderef_2))
  (bind _startgridhitloc (Variables|/Game/Dynamic/BP_CameraPawnController.BP_CameraPawnController_C|GetStartGridHitLoc _camerapawncontrollerref_2))
  (bind _output (CallFunction|XYGridSnap _startgridhitloc))
  (bind _returnvalue (/ _gridsize_2 2.0))
  (bind (_minxy _maxxy) (CallFunction|MinMaxXY (.impactpoint _hitresult) _output))
  (Utilities|Array|Clear (Variables|Default|GetOverlapping))
  (Rendering|SetVisibility (Variables|Default|GetHoverMesh) true false)
  (Utilities|FlowControl|Gate true) ; enters at Open
)

(event Custom|GridClickEnd
  (bind _camerapawncontrollerref (Variables|Default|GetCameraPawnControllerRef))
  (bind _gamemoderef (Variables|Default|GetGameModeRef))
  (bind _camerapawncontrollerref_2 (Variables|Default|GetCameraPawnControllerRef))
  (bind _gamemoderef_2 (Variables|Default|GetGameModeRef))
  (bind _gamemoderef_3 (Variables|Default|GetGameModeRef))
  (bind _camerapawncontrollerref_3 (Variables|Default|GetCameraPawnControllerRef))
  (bind _camerapawncontrollerref_4 (Variables|Default|GetCameraPawnControllerRef))
  (bind _hitresult (Game|Player|GetHitResultUnderCursorbyChannel _camerapawncontrollerref_2 "TraceTypeQuery4" false))
  (bind _startgridhitloc (Variables|/Game/Dynamic/BP_CameraPawnController.BP_CameraPawnController_C|GetStartGridHitLoc _camerapawncontrollerref))
  (bind _gridsize (Variables|/Game/Dynamic/BP_TGUGameMode.BP_TGUGameMode_C|GetGridSize _gamemoderef))
  (bind _gridsize_2 (Variables|/Game/Dynamic/BP_TGUGameMode.BP_TGUGameMode_C|GetGridSize _gamemoderef_2))
  (bind _gridsize_3 (Variables|/Game/Dynamic/BP_TGUGameMode.BP_TGUGameMode_C|GetGridSize _gamemoderef_3))
  (bind _startgridhitloc_2 (Variables|/Game/Dynamic/BP_CameraPawnController.BP_CameraPawnController_C|GetStartGridHitLoc _camerapawncontrollerref_4))
  (bind _endgridhitloc (Variables|/Game/Dynamic/BP_CameraPawnController.BP_CameraPawnController_C|GetEndGridHitLoc _camerapawncontrollerref_3))
  (bind _output (CallFunction|XYGridSnap _startgridhitloc_2))
  (bind (_minxy _maxxy) (CallFunction|MinMaxXY _startgridhitloc _endgridhitloc))
  (bind _returnvalue (/ _gridsize_2 2.0))
  (bind (_minxy_2 _maxxy_2) (CallFunction|MinMaxXY (.impactpoint _hitresult) _output))
  (if (Variables|Default|GetbBuildable)
    (Utilities|FlowControl|Sequence
      (:then_0
        (Rendering|SetVisibility (Variables|Default|GetHoverMesh) false false))
      (:then_1
        (bind _output_get (Variables|Default|SetMinXYLoc _minxy))
        (bind _output_get_2 (Variables|Default|SetMaxXYLoc _maxxy))
        (Development|PrintString (Utilities|String|Append "Start: " (Utilities|String|ToString(Vector) _output_get) "  End: " (Utilities|String|ToString(Vector) _output_get_2)) true true "(R=0.057249,G=1.000000,B=0.000000,A=1.000000)" 1e+01)
        (Variables|Default|SetBuildGridXSquares (+ (Math|Float|Truncate (/ (- (.X (Math|Vector|BreakVector _output_get_2)) (.X (Math|Vector|BreakVector _output_get))) _gridsize_3)) 1))
        (Variables|Default|SetBuildGridYSquares (+ (Math|Float|Truncate (/ (- (.Y (Math|Vector|BreakVector _output_get_2)) (.Y (Math|Vector|BreakVector _output_get))) _gridsize_3)) 1))
        (Variables|Default|SetBuildGridSquares (* (Variables|Default|GetBuildGridXSquares) (Variables|Default|GetBuildGridYSquares)))
        (Game|SpawnActorfromClass "/Game/Dynamic/BP_Foundations.BP_Foundations_C" (Math|Transform|MakeTransform _output_get "0, 0, 0" "1,1,1") "Undefined" 0 0))
      (:then_2
        (Utilities|Array|Clear (Variables|Default|GetOverlapping)))
      (:then_3
        (Utilities|FlowControl|Gate true) ; enters at Close
      ))
    (else
      (Development|PrintString "Invalid Building Selection"))))

(event EventBeginPlay
  (bind _asbp_camera_pawn_controller (Utilities|Casting|CastToBP_CameraPawnController (Game|GetPlayerController 0)))
  (Variables|Default|SetCameraPawnControllerRef _asbp_camera_pawn_controller)
  (bind _asbp_tgugame_mode (Utilities|Casting|CastToBP_TGUGameMode (Game|GetGameMode)))
  (Variables|Default|SetGameModeRef _asbp_tgugame_mode)
  (Utilities|Array|Clear (Variables|Default|GetOverlapping))
  (Variables|Default|SetbBuildable true))

(event Collision|EventActorBeginOverlap
  (params (OtherActor :type Actor%20Object%20Reference))
  (Utilities|Array|AddUnique (Variables|Default|GetOverlapping) OtherActor)
  (if (== (Utilities|Array|Length (Variables|Default|GetOverlapping)) 0)
    (Variables|Default|SetbBuildable true)
    (else
      (Variables|Default|SetbBuildable false))))

(event Collision|EventActorEndOverlap
  (params (OtherActor :type Actor%20Object%20Reference))
  (Utilities|Array|RemoveItem (Variables|Default|GetOverlapping) OtherActor)
  (if (== (Utilities|Array|Length (Variables|Default|GetOverlapping)) 0)
    (Variables|Default|SetbBuildable true)
    (else
      (Variables|Default|SetbBuildable false))))

(event EventTick
  (params (DeltaSeconds :type Float%20%28single-precision%29))
  (bind _gamemoderef (Variables|Default|GetGameModeRef))
  (bind _camerapawncontrollerref (Variables|Default|GetCameraPawnControllerRef))
  (bind _gamemoderef_2 (Variables|Default|GetGameModeRef))
  (bind _camerapawncontrollerref_2 (Variables|Default|GetCameraPawnControllerRef))
  (bind _hitresult (Game|Player|GetHitResultUnderCursorbyChannel _camerapawncontrollerref "TraceTypeQuery4" false))
  (bind _gridsize (Variables|/Game/Dynamic/BP_TGUGameMode.BP_TGUGameMode_C|GetGridSize _gamemoderef))
  (bind _gridsize_2 (Variables|/Game/Dynamic/BP_TGUGameMode.BP_TGUGameMode_C|GetGridSize _gamemoderef_2))
  (bind _startgridhitloc (Variables|/Game/Dynamic/BP_CameraPawnController.BP_CameraPawnController_C|GetStartGridHitLoc _camerapawncontrollerref_2))
  (bind _output (CallFunction|XYGridSnap _startgridhitloc))
  (bind _returnvalue (/ _gridsize_2 2.0))
  (bind (_minxy _maxxy) (CallFunction|MinMaxXY (.impactpoint _hitresult) _output))
  (for _array_element (Variables|Default|GetOverlapping)
    (Development|PrintString (Utilities|GetDisplayName _array_element)))
  (Utilities|FlowControl|Gate true
    (:Exit
      (Utilities|IsValid (.hitactor _hitresult)
        (:Is%20Valid
          (Utilities|FlowControl|Sequence
            (:then_0
              (Variables|Default|SetHoverLoc (.impactpoint _hitresult)))
            (:then_1
              (Variables|Default|SetMinXYHover _minxy))
            (:then_2
              (Variables|Default|SetMaxXYHover (CallFunction|RoundUpMax _maxxy)))
            (:then_3
              (Utilities|FlowControl|Sequence
                (:then_0
                  (Variables|Default|SetHoverGridXSquares (Math|Float|Truncate (/ (- (.x (Variables|Default|GetMaxXYHover)) (.x (Variables|Default|GetMinXYHover))) _gridsize))))
                (:then_1
                  (Variables|Default|SetHoverGridYSquares (Math|Float|Truncate (/ (- (.y (Variables|Default|GetMaxXYHover)) (.y (Variables|Default|GetMinXYHover))) _gridsize))))
                (:then_2
                  (Variables|Default|SetHoverGridSquares (* (Variables|Default|GetHoverGridXSquares) (Variables|Default|GetHoverGridYSquares))))))
            (:then_4
              (Transformation|SetWorldTransform (Variables|Default|GetHoverMesh) (Math|Transform|MakeTransform (- (Math|Vector|MakeVector (.x (/ (+ (CallFunction|XYGridSnap (Variables|Default|GetMaxXYHover)) (CallFunction|XYGridSnap (Variables|Default|GetMinXYHover))) 2.0)) (.y (/ (+ (CallFunction|XYGridSnap (Variables|Default|GetMaxXYHover)) (CallFunction|XYGridSnap (Variables|Default|GetMinXYHover))) 2.0)) (.Z (Math|Vector|BreakVector (Variables|Default|GetHoverLoc)))) (Math|Vector|MakeVector _returnvalue _returnvalue 0.0)) "0, 0, 0" (/ (- (Variables|Default|GetMaxXYHover) (Variables|Default|GetMinXYHover)) (Variables|/Game/Dynamic/BP_TGUGameMode.BP_TGUGameMode_C|GetGridSize (Variables|Default|GetGameModeRef)))) false false)
              (if (Variables|Default|GetbBuildable)
                (Rendering|Material|SetMaterial (Variables|Default|GetHoverMesh) 0 "/Game/Dynamic/M_GridSelect.M_GridSelect")
                (else
                  (Rendering|Material|SetMaterial (Variables|Default|GetHoverMesh) 0 "/Game/Dynamic/M_GridSelectBad.M_GridSelectBad"))))))))))

(fn ConstructionScript)

(fn XYGridSnap
  (params (Input :type Vector))
  (bind (_x _y _z) (Math|Vector|BreakVector Input))
  (bind _gamemoderef (Variables|Default|GetGameModeRef))
  (bind _gamemoderef_2 (Variables|Default|GetGameModeRef))
  (bind _gridsize (Variables|/Game/Dynamic/BP_TGUGameMode.BP_TGUGameMode_C|GetGridSize _gamemoderef_2))
  (bind _gridsize_2 (Variables|/Game/Dynamic/BP_TGUGameMode.BP_TGUGameMode_C|GetGridSize _gamemoderef))
  (return (Math|Vector|MakeVector (+ (* (Math|Float|Floor (/ _x _gridsize_2)) _gridsize_2) (/ _gridsize_2 2.0)) (+ (* (Math|Float|Floor (/ _y _gridsize)) _gridsize) (/ _gridsize 2.0)) _z)))

(fn MinMaxXY
  (params (InA :type Vector) (InB :type Vector))
  (bind (_x _y) (Math|Vector|BreakVector InB))
  (bind (_x_2 _y_2 _z) (Math|Vector|BreakVector InA))
  (return (CallFunction|XYGridSnap (Math|Vector|MakeVector (Math|Float|Min(Float) _x_2 _x) (Math|Float|Min(Float) _y_2 _y) _z)) (CallFunction|XYGridSnap (Math|Vector|MakeVector (Math|Float|Max(Float) _x_2 _x) (Math|Float|Max(Float) _y_2 _y) 0.0))))

(fn RoundUpMax
  (params (InVec :type Vector))
  (bind (_x _y _z) (Math|Vector|BreakVector InVec))
  (bind _gamemoderef (Variables|Default|GetGameModeRef))
  (bind _gridsize (Variables|/Game/Dynamic/BP_TGUGameMode.BP_TGUGameMode_C|GetGridSize _gamemoderef))
  (return (Math|Vector|MakeVector (+ _x _gridsize) (+ _y _gridsize) _z)))