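; BP_Foundations is an actor that lays out a grid of FoundationSquare actors when play begins.
; It takes grid size from BP_TGUGameMode and square count and row width from the last BP_ModularGrid found, then spawns squares row by row from its own location.
; Each square is stored in SquaresArray, and GridComplete is called on them after the loop.
; A downward line trace runs per square, but its result is unused.
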(event EventBeginPlay
  (bind _returnvalue (Transformation|GetActorLocation))
  (bind _asbp_tgugame_mode (Utilities|Casting|CastToBP_TGUGameMode (Game|GetGameMode)))
  (Variables|Default|SetGameModeRef _asbp_tgugame_mode)
  (bind _outactors (Actor|GetAllActorsOfClass "/Game/Dynamic/BP_ModularGrid.BP_ModularGrid_C"))
  (Variables|Default|SetModularGridRef (Utilities|Array|Get(acopy) _outactors (Utilities|Array|LastIndex _outactors)))
  (for _index (range 0 (- (Variables|/Game/Dynamic/BP_ModularGrid.BP_ModularGrid_C|GetBuildGridSquares (Variables|Default|GetModularGridRef)) 1))
    (bind _returnvalue_2 (Game|SpawnActorfromClass "/Game/Dynamic/FoundationSquare.FoundationSquare_C" (Math|Transform|MakeTransform (Math|Vector|MakeVector (+ (.x _returnvalue) (* (Variables|/Game/Dynamic/BP_TGUGameMode.BP_TGUGameMode_C|GetGridSize (Variables|Default|GetGameModeRef)) (Math|Conversions|ToFloat(Integer) (Math|Integer|%(Integer) _index (Variables|/Game/Dynamic/BP_ModularGrid.BP_ModularGrid_C|GetBuildGridXSquares (Variables|Default|GetModularGridRef)))))) (+ (.y _returnvalue) (* (Variables|/Game/Dynamic/BP_TGUGameMode.BP_TGUGameMode_C|GetGridSize (Variables|Default|GetGameModeRef)) (Math|Conversions|ToFloat(Integer) (Math|Float|Floor (/ (Math|Conversions|ToFloat(Integer) _index) (Math|Conversions|ToFloat(Integer) (Variables|/Game/Dynamic/BP_ModularGrid.BP_ModularGrid_C|GetBuildGridXSquares (Variables|Default|GetModularGridRef)))))))) (.z _returnvalue)) "0, 0, 0" "1,1,1") "AlwaysSpawn" 0 0))
    (Utilities|Array|AddUnique (Variables|Default|GetSquaresArray) _returnvalue_2)
    (Collision|LineTraceByChannel "0, 0, 0" "0, 0,-100.000000" "TraceTypeQuery4" false 0 "None"))
  (Default|GridComplete (Variables|Default|GetSquaresArray)))

(fn ConstructionScript)